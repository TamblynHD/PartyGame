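; Levitating block for the Lava Leap level that sinks while the player stands on it and rises back toward its start position afterwards.
; Overlap events on its collision component track the player, and Tick moves the block down by a fixed per-frame step or up by a difficulty speed vector.
; Rising waits for a delay after the player leaves, which a looping timer from BeginPlay keeps lengthening as play goes on.
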(event OnComponentBeginOverlap(LevitatingBlockCollision)
  (params (OverlappedComponent :type Primitive%20Component%20Object%20Reference) (OtherActor :type Actor%20Object%20Reference) (OtherComp :type Primitive%20Component%20Object%20Reference) (OtherBodyIndex :type Integer) (bFromSweep :type Boolean) (SweepResult :type Hit%20Result%20Structure%20%28by%20ref%29))
  ;[1 1 1] On Collision with player set bools
  (Utilities|Casting|CastToThirdPersonCharacter OtherActor)
  (Variables|Default|SetPlayerOnBlock true)
  (Variables|Default|SetCanRise false))

(event OnComponentEndOverlap(LevitatingBlockCollision)
  (params (OverlappedComponent :type Primitive%20Component%20Object%20Reference) (OtherActor :type Actor%20Object%20Reference) (OtherComp :type Primitive%20Component%20Object%20Reference) (OtherBodyIndex :type Integer))
  ;[1 1 1] On Collision with player set bools
  (Utilities|Casting|CastToThirdPersonCharacter OtherActor)
  (Variables|Default|SetPlayerOnBlock false)
  (Utilities|FlowControl|Delay (Variables|Default|GetTimerIncrease))
  (Variables|Default|SetCanRise true))

(event EventBeginPlay
  ;[1 1 1] Being Play : Set start locaiton, every X delay increse timer incerase
  (Variables|Default|SetStartLocation (Transformation|GetWorldLocation (Variables|Default|GetCube)))
  (Utilities|FlowControl|Delay 5.0 :!label _label)
  (Variables|Default|SetTimerIncrease (+ (Variables|Default|GetTimerIncrease) 1.0))
  (goto _label))

(event EventTick
  (params (DeltaSeconds :type Float%20%28single-precision%29))
  (bind _cube (Variables|Default|GetCube))
  (bind _returnvalue (Transformation|GetWorldLocation _cube))
  ;[1 1 1] Tick : if player on block, lower its height, if player not onn, increase height to max of start pos
  (if (Variables|Default|GetPlayerOnBlock)
    (Transformation|SetActorLocation (- (Transformation|GetActorLocation) "0, 0,1.000000") false false)
    (elif (not (Math|Vector|Equal(Vector) _returnvalue (Variables|Default|GetStartLocation) 0.3))
      (if (Variables|Default|GetCanRise)
        (Transformation|SetActorLocation (+ _returnvalue (Variables|Default|GetBlockSpeedDificullty)) false false)))))

(fn ConstructionScript)