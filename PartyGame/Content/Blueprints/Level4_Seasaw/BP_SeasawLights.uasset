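; BP_SeasawLights drives a left and right spot light in the seesaw level from the sea ball's X position.
; Shortly after BeginPlay, it finds the BP_SeaBall actors and sets a loaded flag.
; Each tick it scales the first ball's BallsXLightValue with opposite signs for the two light intensities, so each light responds to opposite sides.
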(event EventBeginPlay
  (Utilities|FlowControl|Delay 0.2)
  (bind _outactors (Actor|GetAllActorsOfClass "/Game/Blueprints/Level4_Seasaw/BP_SeaBall.BP_SeaBall_C"))
  (Variables|Default|SetSeaBallRef _outactors)
  (Variables|Default|SetLoaded true))

(event EventTick
  (params (DeltaSeconds :type Float%20%28single-precision%29))
  (bind _seaballref (Variables|Default|GetSeaBallRef))
  (bind _output (Utilities|Array|Get(acopy) _seaballref))
  (bind _ballsxlightvalue (Variables|/Game/Blueprints/Level4_Seasaw/BP_SeaBall.BP_SeaBall_C|GetBallsXLightValue _output))
  ;[1 1 1] Event Tick : Set spots lights intensity dependent on balls X location
  (if (Variables|Default|GetLoaded)
    (Utilities|FlowControl|Sequence
      (:then_0
        (Rendering|Components|Light|SetIntensity (Variables|Default|GetLeftSpotLight) (* _ballsxlightvalue -1e+02)))
      (:then_1
        (Rendering|Components|Light|SetIntensity (Variables|Default|GetRightSpotLight) (* _ballsxlightvalue 1e+02))))))

(fn ConstructionScript)