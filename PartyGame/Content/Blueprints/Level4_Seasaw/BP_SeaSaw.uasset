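; BP_SeaSaw is a seesaw actor that tilts left or right according to the sign of SeaSawButtonLevel.
; BeginPlay stores the mesh's starting rotation and derives both pitch limits from MaxDegree through SetMaxRotators.
; Each tick steps the pitch by RotationSpeed until it is within a small tolerance of that side's limit, without delta-time scaling.
; A level of zero holds the current tilt.
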(event EventTick
  (params (DeltaSeconds :type Float%20%28single-precision%29))
  ;[1 1 1] Event Tick : Dependent on level, rotate left and right
  (if (<= (Variables|Default|GetSeaSawButtonLevel) -1)
    (if (not (Math|Rotator|Equal(Rotator) (Variables|Default|GetTargetRotation) (Variables|Default|GetLeftMaxRot) 3.0))
      (Transformation|SetWorldRotation (Variables|Default|GetSeasawmain) (Math|Rotator|MakeRotator (.Roll (Math|Rotator|BreakRotator (Variables|Default|GetTargetRotation))) (+ (.Pitch (Math|Rotator|BreakRotator (Variables|Default|GetTargetRotation))) (Variables|Default|GetRotationSpeed)) (.Yaw (Math|Rotator|BreakRotator (Variables|Default|GetTargetRotation)))) false false)
      (Variables|Default|SetTargetRotation (Math|Rotator|MakeRotator (.Roll (Math|Rotator|BreakRotator (Variables|Default|GetTargetRotation))) (+ (.Pitch (Math|Rotator|BreakRotator (Variables|Default|GetTargetRotation))) (Variables|Default|GetRotationSpeed)) (.Yaw (Math|Rotator|BreakRotator (Variables|Default|GetTargetRotation))))))
    (elif (>= (Variables|Default|GetSeaSawButtonLevel) 1)
      (if (not (Math|Rotator|Equal(Rotator) (Variables|Default|GetTargetRotation) (Variables|Default|GetRightMaxRot) 3.0))
        (Transformation|SetWorldRotation (Variables|Default|GetSeasawmain) (Math|Rotator|MakeRotator (.Roll (Math|Rotator|BreakRotator (Variables|Default|GetTargetRotation))) (- (.Pitch (Math|Rotator|BreakRotator (Variables|Default|GetTargetRotation))) (Variables|Default|GetRotationSpeed)) (.Yaw (Math|Rotator|BreakRotator (Variables|Default|GetTargetRotation)))) false false)
        (Variables|Default|SetTargetRotation (Math|Rotator|MakeRotator (.Roll (Math|Rotator|BreakRotator (Variables|Default|GetTargetRotation))) (- (.Pitch (Math|Rotator|BreakRotator (Variables|Default|GetTargetRotation))) (Variables|Default|GetRotationSpeed)) (.Yaw (Math|Rotator|BreakRotator (Variables|Default|GetTargetRotation)))))))))

(event EventBeginPlay
  ;[1 1 1] Begin Play : Set base rotations
  (bind _output_get (Variables|Default|SetTargetRotation (Transformation|GetWorldRotation (Variables|Default|GetSeasawmain))))
  (bind _output_get_2 (Variables|Default|SetStartRotation _output_get))
  (Variables|Default|SetLeftMaxRot (.Left (Utilities|SetMaxRotators _output_get_2 (Variables|Default|GetMaxDegree))))
  (Variables|Default|SetRightMaxRot (.Right (Utilities|SetMaxRotators _output_get_2 (Variables|Default|GetMaxDegree)))))

(fn ConstructionScript)