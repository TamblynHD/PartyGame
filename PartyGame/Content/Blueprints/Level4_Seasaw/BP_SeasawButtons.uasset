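; A pair of left and right floor buttons that the player steps on to tilt the level's BP_SeaSaw.
; On Begin Play it randomizes each button's X position, derives raised and lowered positions, finds the seesaw and sets the starting state from UpStart.
; When the player overlaps a raised button's box, that button drops, the other rises, and the seesaw's button level moves up for left or down for right.
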(event OnComponentBeginOverlap(LeftBoxCollision)
  (params (OverlappedComponent :type Primitive%20Component%20Object%20Reference) (OtherActor :type Actor%20Object%20Reference) (OtherComp :type Primitive%20Component%20Object%20Reference) (OtherBodyIndex :type Integer) (bFromSweep :type Boolean) (SweepResult :type Hit%20Result%20Structure%20%28by%20ref%29))
  (bind _seasawref (Variables|Default|GetSeaSawRef))
  ;[1 1 1] On Player collision, push respective button down and oppisite one up.  Set seasaw level for rotation
  (Utilities|Casting|CastToThirdPersonCharacter OtherActor)
  (if (not (Variables|Default|GetLeftSidePushed))
    (Variables|Default|SetLeftSidePushed true)
    (Transformation|SetWorldLocation (Variables|Default|GetButtonRight) (Variables|Vectors|GetRightHighestButPos) false false)
    (Transformation|SetWorldLocation (Variables|Default|GetButtonLeft) (Variables|Vectors|GetLeftLowestButPos) false false)
    (Variables|Default|SetRightSidePushed false)
    (Variables|/Game/Blueprints/Level4_Seasaw/BP_SeaSaw.BP_SeaSaw_C|SetSeaSawButtonLevel _seasawref (+ (Variables|/Game/Blueprints/Level4_Seasaw/BP_SeaSaw.BP_SeaSaw_C|GetSeaSawButtonLevel _seasawref) 1))))

(event OnComponentBeginOverlap(RightBoxCollision)
  (params (OverlappedComponent :type Primitive%20Component%20Object%20Reference) (OtherActor :type Actor%20Object%20Reference) (OtherComp :type Primitive%20Component%20Object%20Reference) (OtherBodyIndex :type Integer) (bFromSweep :type Boolean) (SweepResult :type Hit%20Result%20Structure%20%28by%20ref%29))
  (bind _seasawref (Variables|Default|GetSeaSawRef))
  ;[1 1 1] On Player collision, push respective button down and oppisite one up.  Set seasaw level for rotation
  (Utilities|Casting|CastToThirdPersonCharacter OtherActor)
  (if (not (Variables|Default|GetRightSidePushed))
    (Variables|Default|SetRightSidePushed true)
    (Transformation|SetWorldLocation (Variables|Default|GetButtonLeft) (Variables|Vectors|GetLeftHighestButPos) false false)
    (Transformation|SetWorldLocation (Variables|Default|GetButtonRight) (Variables|Vectors|GetRightLowestButPos) false false)
    (Variables|Default|SetLeftSidePushed false)
    (Variables|/Game/Blueprints/Level4_Seasaw/BP_SeaSaw.BP_SeaSaw_C|SetSeaSawButtonLevel _seasawref (- (Variables|/Game/Blueprints/Level4_Seasaw/BP_SeaSaw.BP_SeaSaw_C|GetSeaSawButtonLevel _seasawref) 1))))

(event EventBeginPlay
  ;[1 1 1] Begin Play : Set button vectors, create a ref to the seasaw in level and activate a button ready for use
  (CallFunction|SetButtonVectors)
  (bind _outactors (Actor|GetAllActorsOfClass "/Game/Blueprints/Level4_Seasaw/BP_SeaSaw.BP_SeaSaw_C"))
  (Variables|Default|SetSeaSawRef (Utilities|Array|Get(acopy) _outactors))
  (if (Variables|Default|GetUpStart)
    (Transformation|SetWorldLocation (Variables|Default|GetButtonLeft) (Variables|Vectors|GetLeftHighestButPos) false false)
    (Variables|Default|SetRightSidePushed true)
    (Transformation|SetWorldLocation (Variables|Default|GetButtonRight) (Variables|Vectors|GetRightLowestButPos) false false)
    (else
      (Transformation|SetWorldLocation (Variables|Default|GetButtonRight) (Variables|Vectors|GetRightHighestButPos) false false)
      (Variables|Default|SetLeftSidePushed true)
      (Transformation|SetWorldLocation (Variables|Default|GetButtonLeft) (Variables|Vectors|GetLeftLowestButPos) false false))))

(fn ConstructionScript)

(fn SetButtonVectors
  (bind _buttonheightscale (Variables|Vectors|GetButtonHeightScale))
  ;[1 1 1] Get buttons middle location from where they start
  (Variables|Vectors|SetLeftButStartPos (Transformation|GetWorldLocation (Variables|Default|GetButtonLeft)))
  (Variables|Vectors|SetRightButStartPos (Transformation|GetWorldLocation (Variables|Default|GetButtonRight)))
  ;[1 1 1] Randomize X axis spawn location
  (Transformation|SetWorldLocation (Variables|Default|GetButtonLeft) (Math|Vector|MakeVector (- (.X (Math|Vector|BreakVector (Variables|Vectors|GetLeftButStartPos))) (Math|Random|RandomFloatinRange (Variables|Default|GetMinXRange) (Variables|Default|GetMaxXRange))) (.Y (Math|Vector|BreakVector (Variables|Vectors|GetLeftButStartPos))) (.Z (Math|Vector|BreakVector (Variables|Vectors|GetLeftButStartPos)))) false false)
  (Transformation|SetWorldLocation (Variables|Default|GetButtonRight) (Math|Vector|MakeVector (+ (.X (Math|Vector|BreakVector (Variables|Vectors|GetRightButStartPos))) (Math|Random|RandomFloatinRange (Variables|Default|GetMinXRange) (Variables|Default|GetMaxXRange))) (.Y (Math|Vector|BreakVector (Variables|Vectors|GetRightButStartPos))) (.Z (Math|Vector|BreakVector (Variables|Vectors|GetRightButStartPos)))) false false)
  ;[1 1 1] Recollect button location
  (Variables|Vectors|SetLeftButStartPos (Transformation|GetWorldLocation (Variables|Default|GetButtonLeft)))
  (Variables|Vectors|SetRightButStartPos (Transformation|GetWorldLocation (Variables|Default|GetButtonRight)))
  ;[1 1 1] Plus or minus start position to determine up and down positions
  (Variables|Vectors|SetLeftLowestButPos (- (Variables|Vectors|GetLeftButStartPos) _buttonheightscale))
  (Variables|Vectors|SetLeftHighestButPos (+ (Variables|Vectors|GetLeftButStartPos) _buttonheightscale))
  (Variables|Vectors|SetRightLowestButPos (- (Variables|Vectors|GetRightButStartPos) _buttonheightscale))
  (Variables|Vectors|SetRightHighestButPos (+ (Variables|Vectors|GetRightButStartPos) _buttonheightscale)))