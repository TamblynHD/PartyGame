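; BP_BigPengu is a penguin actor that slides along world X at a random speed and destroys itself ten seconds after spawning.
; BeginPlay picks the speed, and Tick adds it to the location each frame without sweep or delta-time scaling.
; When its front box overlaps a BP_Pengu, it speeds that pengu up and slows itself down, like a simple bump.
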(event OnComponentBeginOverlap(FrontBoxCollision)
  (params (OverlappedComponent :type Primitive%20Component%20Object%20Reference) (OtherActor :type Actor%20Object%20Reference) (OtherComp :type Primitive%20Component%20Object%20Reference) (OtherBodyIndex :type Integer) (bFromSweep :type Boolean) (SweepResult :type Hit%20Result%20Structure%20%28by%20ref%29))
  ;[1 1 1] On collision with pengu infront change speed of both pengus
  (bind _asbp_pengu (Utilities|Casting|CastToBP_Pengu OtherActor))
  (Variables|/Game/Blueprints/BP_Pengu.BP_Pengu_C|SetPenguSpeed _asbp_pengu (+ (Variables|/Game/Blueprints/BP_Pengu.BP_Pengu_C|GetPenguSpeed _asbp_pengu) "2.000000, 0, 0"))
  (Variables|Default|SetPenguSpeed (- (Variables|Default|GetPenguSpeed) "1.000000, 0, 0")))

(event Custom|SetPenguSpeed
  ;[1 1 1] Set random speed for Pengus
  (Variables|Default|SetPenguSpeed (Math|Vector|MakeVector (Math|Random|RandomFloatinRange 2.0 5.0) 0.0 0.0)))

(event EventBeginPlay
  ;[1 1 1] Begin Play : After a delay destroy actor (Cleanup)
  (CallFunction|SetPenguSpeed)
  (Utilities|FlowControl|Delay 1e+01)
  (Actor|DestroyActor))

(event EventTick
  (params (DeltaSeconds :type Float%20%28single-precision%29))
  ;[1 1 1] Tick : Every tick move actor along X at pengu's speed
  (Transformation|SetActorLocation (+ (.Location (Math|Transform|BreakTransform (Transformation|GetWorldTransform (Variables|Default|GetDefaultSceneRoot)))) (Variables|Default|GetPenguSpeed)) false false))

(fn ConstructionScript)