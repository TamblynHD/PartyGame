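; Spawner actor for the Level 5 door wall that keeps spawning random doors at its Arrow component's location.
; BeginPlay requires a BP_GameMode cast, waits briefly, then runs an endless delay loop calling SpawnDoor, which picks one of four DoorArray classes.
; The loop shortens DoorSpawnTimer after each spawn until it bottoms out at about a second, so doors arrive increasingly fast.
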(event Custom|SpawnDoor
  (Game|SpawnActorfromClass (Utilities|Array|Get(acopy) (Variables|Default|GetDoorArray) (Math|Random|RandomInteger 4)) (Math|Transform|MakeTransform (Transformation|GetWorldLocation (Variables|Default|GetArrow))) "Undefined" 0 0))

(event EventBeginPlay
  (bind _asbp_game_mode (Utilities|Casting|CastToBP_GameMode (Game|GetGameMode)))
  (Utilities|FlowControl|Delay 2.0)
  (CallFunction|SpawnDoor)
  (Utilities|FlowControl|Delay (Variables|Default|GetDoorSpawnTimer) :!label _label)
  (CallFunction|SpawnDoor)
  (if (<= (Variables|Default|GetDoorSpawnTimer) 1.0)
    (goto _label)
    (else
      (Variables|Default|SetDoorSpawnTimer (- (Variables|Default|GetDoorSpawnTimer) 0.5))
      (goto _label))))

(fn ConstructionScript)