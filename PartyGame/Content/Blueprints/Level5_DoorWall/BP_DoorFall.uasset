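; BP_DoorFall is an overlap trigger actor in the Level 5 door wall that makes doors fall and kills the player.
; DeathCollision sets Dead on an overlapping ThirdPersonCharacter.
; DoorFallcollision1 sets Falling on an overlapping BP_Door1.
; DoorFallcollision2 to 4 follow the same cast-and-set pattern, but their cast target classes are empty, apparently missing references.
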(event OnComponentBeginOverlap(DoorFallcollision1)
  (params (OverlappedComponent :type Primitive%20Component%20Object%20Reference) (OtherActor :type Actor%20Object%20Reference) (OtherComp :type Primitive%20Component%20Object%20Reference) (OtherBodyIndex :type Integer) (bFromSweep :type Boolean) (SweepResult :type Hit%20Result%20Structure%20%28by%20ref%29))
  (bind _asbp_door_1 (Utilities|Casting|CastToBP_Door1 OtherActor))
  (Variables|/Game/Blueprints/Level5_DoorWall/BP_Door1.BP_Door1_C|SetFalling _asbp_door_1 true))

(event OnComponentBeginOverlap(DoorFallcollision2)
  (params (OverlappedComponent :type Primitive%20Component%20Object%20Reference) (OtherActor :type Actor%20Object%20Reference) (OtherComp :type Primitive%20Component%20Object%20Reference) (OtherBodyIndex :type Integer) (bFromSweep :type Boolean) (SweepResult :type Hit%20Result%20Structure%20%28by%20ref%29))
  (bind _asbp_door_2 (Utilities|Casting|CastTo OtherActor))
  (Variables|Default|SetFalling _asbp_door_2 true))

(event OnComponentBeginOverlap(DoorFallcollision3)
  (params (OverlappedComponent :type Primitive%20Component%20Object%20Reference) (OtherActor :type Actor%20Object%20Reference) (OtherComp :type Primitive%20Component%20Object%20Reference) (OtherBodyIndex :type Integer) (bFromSweep :type Boolean) (SweepResult :type Hit%20Result%20Structure%20%28by%20ref%29))
  (bind _asbp_door_3 (Utilities|Casting|CastTo OtherActor))
  (Variables|Default|SetFalling _asbp_door_3 true))

(event OnComponentBeginOverlap(DoorFallcollision4)
  (params (OverlappedComponent :type Primitive%20Component%20Object%20Reference) (OtherActor :type Actor%20Object%20Reference) (OtherComp :type Primitive%20Component%20Object%20Reference) (OtherBodyIndex :type Integer) (bFromSweep :type Boolean) (SweepResult :type Hit%20Result%20Structure%20%28by%20ref%29))
  (bind _asbp_door_4 (Utilities|Casting|CastTo OtherActor))
  (Variables|Default|SetFalling _asbp_door_4 true))

(event OnComponentBeginOverlap(DeathCollision)
  (params (OverlappedComponent :type Primitive%20Component%20Object%20Reference) (OtherActor :type Actor%20Object%20Reference) (OtherComp :type Primitive%20Component%20Object%20Reference) (OtherBodyIndex :type Integer) (bFromSweep :type Boolean) (SweepResult :type Hit%20Result%20Structure%20%28by%20ref%29))
  (bind _asthird_person_character (Utilities|Casting|CastToThirdPersonCharacter OtherActor))
  (Variables|/Game/ThirdPersonBP/Blueprints/ThirdPersonCharacter.ThirdPersonCharacter_C|SetDead _asthird_person_character true))

(event EventBeginPlay)

(event EventTick
  (params (DeltaSeconds :type Float%20%28single-precision%29)))

(fn ConstructionScript)