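; BP_Door4 is a moving door actor for the Level 5 door wall.
; Every Tick it offsets the actor from its root's world location by DoorFallinSpeed when Falling is set, otherwise by DoorSpeed.
; The movement is a per-frame step without sweep or delta-time scaling, so its speed depends on frame rate.
; Nothing in its graphs changes Falling.
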(event EventTick
  (params (DeltaSeconds :type Float%20%28single-precision%29))
  (if (Variables|Default|GetFalling)
    (Transformation|SetActorLocation (+ (.Location (Math|Transform|BreakTransform (Transformation|GetWorldTransform (Variables|Default|GetDefaultSceneRoot)))) (Variables|Default|GetDoorFallinSpeed)) false false)
    (else
      (Transformation|SetActorLocation (+ (.Location (Math|Transform|BreakTransform (Transformation|GetWorldTransform (Variables|Default|GetDefaultSceneRoot)))) (Variables|Default|GetDoorSpeed)) false false))))

(fn ConstructionScript)