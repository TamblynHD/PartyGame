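; BP_Pengu is a penguin actor in the PushyPengu level that slides along at a per-tick offset and destroys itself after a delay.
; SetSpeed randomly picks a speed tier on BeginPlay, though its medium branch assigns MediumSpeed to itself, leaving PenguSpeed unchanged.
; Front-box overlaps with another pengu bump that one up a tier via SpeedTest and drop this one via UnSpeedTest.
; The big-pengu overlap event is empty.
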(event OnComponentBeginOverlap(FrontBoxCollision)
  (params (OverlappedComponent :type Primitive%20Component%20Object%20Reference) (OtherActor :type Actor%20Object%20Reference) (OtherComp :type Primitive%20Component%20Object%20Reference) (OtherBodyIndex :type Integer) (bFromSweep :type Boolean) (SweepResult :type Hit%20Result%20Structure%20%28by%20ref%29))
  (bind _self self)
  ;[1 1 1 0.3619] On collision with pengu infront change speed of both pengus
  (bind _asbp_pengu (Utilities|Casting|CastToBP_Pengu OtherActor))
  (CallFunction|SpeedTest _asbp_pengu (Variables|BP_Pengu_C|GetPenguSpeed _asbp_pengu) _asbp_pengu)
  (CallFunction|UnSpeedTest _self (Variables|Default|GetPenguSpeed) _self))

(event OnComponentBeginOverlap(FrontBigCollision)
  (params (OverlappedComponent :type Primitive%20Component%20Object%20Reference) (OtherActor :type Actor%20Object%20Reference) (OtherComp :type Primitive%20Component%20Object%20Reference) (OtherBodyIndex :type Integer) (bFromSweep :type Boolean) (SweepResult :type Hit%20Result%20Structure%20%28by%20ref%29))
  ;[1 1 1] On collision with big pengu infront change speed of both pengus
)

(event Custom|SetPenguSpeed
  ;[1 1 1] Set random speed for Pengus
)

(event EventBeginPlay
  ;[1 1 1] Begin Play : After a delay destroy actor (Cleanup)
  (Utilities|SetSpeed
    (:out
      (Utilities|FlowControl|Delay 1e+01)
      (Actor|DestroyActor))))

(event EventTick
  (params (DeltaSeconds :type Float%20%28single-precision%29))
  ;[1 1 1] Tick : Every tick move actor along X at pengu's speed
  (Transformation|SetActorLocation (+ (.Location (Math|Transform|BreakTransform (Transformation|GetWorldTransform (Variables|Default|GetDefaultSceneRoot)))) (Variables|Default|GetPenguSpeed)) false false))

(fn ConstructionScript)

(fn SpeedTest
  (params (A :type Vector) (Target :type BP%20Pengu%20Object%20Reference))
  (if (Class|KismetMathLibrary|EqualExactlyVectorVector A (Variables|Default|GetLowSpeed))
    (Variables|BP_Pengu_C|SetPenguSpeed Target (Variables|Default|GetMediumSpeed))
    (elif (Class|KismetMathLibrary|EqualExactlyVectorVector A (Variables|Default|GetMediumSpeed))
      (Variables|BP_Pengu_C|SetPenguSpeed Target (Variables|Default|GetHighSpeed))
      (elif (Class|KismetMathLibrary|EqualExactlyVectorVector A (Variables|Default|GetHighSpeed))
        (Variables|BP_Pengu_C|SetPenguSpeed Target (Variables|Default|GetVeryHighSpeed))))))

(fn UnSpeedTest
  (params (A :type Vector) (Target :type BP%20Pengu%20Object%20Reference))
  (if (Class|KismetMathLibrary|EqualExactlyVectorVector A (Variables|Default|GetVeryHighSpeed))
    (Variables|BP_Pengu_C|SetPenguSpeed Target (Variables|Default|GetHighSpeed))
    (elif (Class|KismetMathLibrary|EqualExactlyVectorVector A (Variables|Default|GetHighSpeed))
      (Variables|BP_Pengu_C|SetPenguSpeed Target (Variables|Default|GetMediumSpeed))
      (elif (Class|KismetMathLibrary|EqualExactlyVectorVector A (Variables|Default|GetMediumSpeed))
        (Variables|BP_Pengu_C|SetPenguSpeed Target (Variables|Default|GetLowSpeed))))))