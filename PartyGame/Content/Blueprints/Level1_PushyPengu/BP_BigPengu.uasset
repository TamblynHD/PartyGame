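; BP_BigPengu is a large penguin actor in the Pushy Pengu level that moves along its path and destroys itself after a fixed lifetime.
; Tick adds the BigPenguSpeed vector to its location without sweep or delta-time scaling, so movement depends on frame rate.
; A front box overlap copies that speed onto any BP_Pengu it hits.
; Random speed setup and big-to-big speed exchange are disconnected, leaving those events empty.
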(event OnComponentBeginOverlap(FrontBoxCollision)
  (params (OverlappedComponent :type Primitive%20Component%20Object%20Reference) (OtherActor :type Actor%20Object%20Reference) (OtherComp :type Primitive%20Component%20Object%20Reference) (OtherBodyIndex :type Integer) (bFromSweep :type Boolean) (SweepResult :type Hit%20Result%20Structure%20%28by%20ref%29))
  (bind _asbp_pengu (Utilities|Casting|CastToBP_Pengu OtherActor))
  (Variables|/Game/Blueprints/Level1_PushyPengu/BP_Pengu.BP_Pengu_C|SetPenguSpeed _asbp_pengu (Variables|Default|GetBigPenguSpeed)))

(event OnComponentBeginOverlap(FrontBigBoxCollision)
  (params (OverlappedComponent :type Primitive%20Component%20Object%20Reference) (OtherActor :type Actor%20Object%20Reference) (OtherComp :type Primitive%20Component%20Object%20Reference) (OtherBodyIndex :type Integer) (bFromSweep :type Boolean) (SweepResult :type Hit%20Result%20Structure%20%28by%20ref%29))
  ;[1 1 1] On collision with big pengu infront change speed of both pengus
)

(event Custom|SetPenguSpeed
  ;[1 1 1] Set random speed for Pengus
)

(event EventBeginPlay
  ;[1 1 1] Begin Play : After a delay destroy actor (Cleanup)
  (Utilities|FlowControl|Delay 1e+01)
  (Actor|DestroyActor))

(event EventTick
  (params (DeltaSeconds :type Float%20%28single-precision%29))
  ;[1 1 1] Tick : Every tick move actor along X at pengu's speed
  (Transformation|SetActorLocation (+ (.Location (Math|Transform|BreakTransform (Transformation|GetWorldTransform (Variables|Default|GetDefaultSceneRoot)))) (Variables|Default|GetBigPenguSpeed)) false false))

(fn ConstructionScript)