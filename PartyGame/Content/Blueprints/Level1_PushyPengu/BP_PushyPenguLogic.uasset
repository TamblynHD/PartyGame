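; Level 1 PushyPengu spawner that keeps dropping random penguin types into the level.
; On BeginPlay it gathers ten arrow components into an array, waits briefly, then loops on a PenguRespawnTimer delay.
; Each pass spawns a random PenguTypeArray class at a random arrow's location with zero rotation.
; The random index range of 9 covers 0 to 8, so Arrow9 is never picked.
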(event Custom|PenguAddArray
  ;[1 1 1] Make Array of arrows for pengu spawns
  (Variables|Default|SetArrowsArray (Utilities|Array|MakeArray (Variables|Arrows|GetArrow) (Variables|Arrows|GetArrow1) (Variables|Arrows|GetArrow2) (Variables|Arrows|GetArrow3) (Variables|Arrows|GetArrow4) (Variables|Arrows|GetArrow5) (Variables|Arrows|GetArrow6) (Variables|Arrows|GetArrow7) (Variables|Arrows|GetArrow8) (Variables|Default|GetArrow9))))

(event Custom|SpawnPengus
  ;[1 1 1] Spawn Pengus
  (Game|SpawnActorfromClass (Utilities|Array|Get(acopy) (Variables|Default|GetPenguTypeArray) (Math|Random|RandomInteger 8)) (Math|Transform|MakeTransform (Transformation|GetWorldLocation (Utilities|Array|Get(acopy) (Variables|Default|GetArrowsArray) (Math|Random|RandomInteger 9)))) "Undefined" 0 0))

(event EventBeginPlay
  ;[1 1 1] Begin Play : set pengu array, then every respwan timer seconds spawn a pengu
  (CallFunction|PenguAddArray)
  (Utilities|FlowControl|Delay 1.0)
  (CallFunction|SpawnPengus :!label _label)
  (Utilities|FlowControl|Delay (Variables|Default|GetPenguRespawnTimer))
  (goto _label))

(fn ConstructionScript)