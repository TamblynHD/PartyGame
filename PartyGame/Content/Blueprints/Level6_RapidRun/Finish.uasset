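; Finish actor for the Rapid Run level whose cube starts sinking when the player character enters its trigger.
; The Box overlap casts to ThirdPersonCharacter and sets a CanFall flag that is never cleared.
; While the flag is set, Tick lowers the Cube by a fixed step each frame without sweep, so the speed depends on frame rate and the descent has no end.
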(event OnComponentBeginOverlap(Box)
  (params (OverlappedComponent :type Primitive%20Component%20Object%20Reference) (OtherActor :type Actor%20Object%20Reference) (OtherComp :type Primitive%20Component%20Object%20Reference) (OtherBodyIndex :type Integer) (bFromSweep :type Boolean) (SweepResult :type Hit%20Result%20Structure%20%28by%20ref%29))
  (Utilities|Casting|CastToThirdPersonCharacter OtherActor)
  (Variables|Default|SetCanFall true))

(event EventTick
  (params (DeltaSeconds :type Float%20%28single-precision%29))
  (bind _cube (Variables|Default|GetCube))
  (bind _returnvalue (Transformation|GetWorldLocation _cube))
  (bind (_x _y _z) (Math|Vector|BreakVector _returnvalue))
  (if (Variables|Default|GetCanFall)
    (Transformation|SetWorldLocation _cube (Math|Vector|MakeVector _x _y (- _z 2.0)) false false)))

(fn ConstructionScript)