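; EP_QuestionLogic holds the question pool for the Level 2 QuizBizz quiz and picks the current question at random.
; On BeginPlay it fills QuestionArray from five question variables, then calls RanomQuestion to set CurrentQuestion.
; The random index spans only the first four entries, so the last question is never selected.
; The BP_AnswerBlock lookup is unwired, and QuestionNumber and QuestionVariety are unused.
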(event Custom|RanomQuestion
  (Variables|Questions|SetCurrentQuestion (Utilities|Array|Get(acopy) (Variables|Questions|GetQuestionArray) (Math|Random|RandomInteger 4))))

(event EventBeginPlay
  ;[1 1 1] Set Up
  (Variables|Questions|SetQuestionArray (Utilities|Array|MakeArray (Variables|Questions|GetQuestion) (Variables|Questions|GetQuestion_0) (Variables|Questions|GetQuestion_1) (Variables|Questions|GetQuestion_2) (Variables|Questions|GetQuestion_3)))
  (CallFunction|RanomQuestion))

(fn ConstructionScript)