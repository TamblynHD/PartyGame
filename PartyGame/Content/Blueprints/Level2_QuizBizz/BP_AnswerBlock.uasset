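; BP_AnswerBlock is an answer block in the Level 2 QuizBizz quiz that displays answer options through a TextRender.
; Every Tick it finds EP_QuestionLogic and all answer blocks, then compares CurrentQuestion against hardcoded question strings to pick four answers.
; For the first question it writes the answers to the first four blocks by array index, so each block updates the whole set.
; The second question only sets the answer variables without updating any text.
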(event EventTick
  (params (DeltaSeconds :type Float%20%28single-precision%29))
  (bind _outactors (Actor|GetAllActorsOfClass "/Game/Blueprints/Level2_QuizBizz/EP_QuestionLogic.EP_QuestionLogic_C"))
  (bind _outactors_2 (Actor|GetAllActorsOfClass "BP_AnswerBlock_C"))
  (if (Utilities|Enum|Equal(Enum) (Variables|/Game/Blueprints/Level2_QuizBizz/EP_QuestionLogic.EP_QuestionLogic_C|GetCurrentQuestion (Utilities|Array|Get(acopy) _outactors)) "Whats Pie?")
    (bind _output_get (Variables|Default|SetAnswer1 "3"))
    (Rendering|Components|TextRender|SetText (Variables|BP_AnswerBlock_C|GetTextRender (Utilities|Array|Get(acopy) _outactors_2)) (Utilities|Text|ToText(String) _output_get))
    (bind _output_get_2 (Variables|Default|SetAnswer2 "4"))
    (Rendering|Components|TextRender|SetText (Variables|BP_AnswerBlock_C|GetTextRender (Utilities|Array|Get(acopy) _outactors_2 1)) (Utilities|Text|ToText(String) _output_get_2))
    (bind _output_get_3 (Variables|Default|SetAnswer3 "6"))
    (Rendering|Components|TextRender|SetText (Variables|BP_AnswerBlock_C|GetTextRender (Utilities|Array|Get(acopy) _outactors_2 2)) (Utilities|Text|ToText(String) _output_get_3))
    (bind _output_get_4 (Variables|Default|SetAnswer4 "block"))
    (Rendering|Components|TextRender|SetText (Variables|BP_AnswerBlock_C|GetTextRender (Utilities|Array|Get(acopy) _outactors_2 3)) (Utilities|Text|ToText(String) _output_get_4))
    (elif (Utilities|Enum|Equal(Enum) (Variables|/Game/Blueprints/Level2_QuizBizz/EP_QuestionLogic.EP_QuestionLogic_C|GetCurrentQuestion (Utilities|Array|Get(acopy) _outactors)) "Whats wrong?")
      (Variables|Default|SetAnswer1 "a")
      (Variables|Default|SetAnswer2 "b")
      (Variables|Default|SetAnswer3 "c")
      (Variables|Default|SetAnswer4 "d"))))

(fn ConstructionScript)