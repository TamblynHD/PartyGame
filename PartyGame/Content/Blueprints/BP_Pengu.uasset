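; BP_Pengu is a moving actor that removes itself ten seconds after it spawns.
; Each Tick it adds the PenguSpeed vector to its root's location, commented as movement along X, without sweep or delta-time scaling, so speed depends on frame rate.
; The SetPenguSpeed event zeroes that vector, halting the movement.
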(event Custom|SetPenguSpeed
  (Variables|Default|SetPenguSpeed "0, 0, 0"))

(event EventBeginPlay
  ;[1 1 1] Begin Play : After a delay destroy actor (Cleanup)
  (Utilities|FlowControl|Delay 1e+01)
  (Actor|DestroyActor))

(event EventTick
  (params (DeltaSeconds :type Float%20%28single-precision%29))
  ;[1 1 1] Tick : Every tick move actor along X at pengu's speed
  (Transformation|SetActorLocation (+ (.Location (Math|Transform|BreakTransform (Transformation|GetWorldTransform (Variables|Default|GetDefaultSceneRoot)))) (Variables|Default|GetPenguSpeed)) false false))

(fn ConstructionScript)