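; Results-podium block that shows one player's score and moves to a height based on it.
; On BeginPlay it reads the score for its PlayerNumber from BPI_GameInstance, sets the text and derives a target height.
; After startup delays, Tick steps the cube's Z until it nears the target; a zero score reverses the direction to sink it.
; Ranking functions and place-height vectors exist but do not drive the movement.
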(event Custom|RaisePodium
  (bind _podiumcube (Variables|Default|GetPodiumCube))
  (bind _returnvalue (Transformation|GetWorldLocation _podiumcube))
  (bind (_x _y _z) (Math|Vector|BreakVector _returnvalue))
  ;[1 1 1] Raise Podium
  (Transformation|SetWorldLocation _podiumcube (Math|Vector|MakeVector _x _y (+ _z (Variables|Default|GetPodiumLiftSpeed))) false false))

(event Custom|HeightCheck
  (bind _playernumber (Variables|Default|GetPlayerNumber))
  ;[1 1 1] Height Check
  (bind _asbpi_game_instance (Utilities|Casting|CastToBPI_GameInstance (Game|GetGameInstance)))
  (if (== _playernumber 0)
    (CallFunction|HeightSet (Variables|/Game/Blueprints/BPI_GameInstance.BPI_GameInstance_C|GetPlayer1Score _asbpi_game_instance))
    (Rendering|Components|TextRender|SetText (Variables|Default|GetTextRender) (Utilities|Text|ToText(Integer) (Variables|/Game/Blueprints/BPI_GameInstance.BPI_GameInstance_C|GetPlayer1Score _asbpi_game_instance)))
    (elif (== _playernumber 1)
      (CallFunction|HeightSet (Variables|/Game/Blueprints/BPI_GameInstance.BPI_GameInstance_C|GetPlayer2Score _asbpi_game_instance))
      (Rendering|Components|TextRender|SetText (Variables|Default|GetTextRender) (Utilities|Text|ToText(Integer) (Variables|/Game/Blueprints/BPI_GameInstance.BPI_GameInstance_C|GetPlayer2Score _asbpi_game_instance)))
      (elif (== _playernumber 2)
        (CallFunction|HeightSet (Variables|/Game/Blueprints/BPI_GameInstance.BPI_GameInstance_C|GetPlayer3Score _asbpi_game_instance))
        (Rendering|Components|TextRender|SetText (Variables|Default|GetTextRender) (Utilities|Text|ToText(Integer) (Variables|/Game/Blueprints/BPI_GameInstance.BPI_GameInstance_C|GetPlayer3Score _asbpi_game_instance)))
        (elif (== _playernumber 3)
          (CallFunction|HeightSet (Variables|/Game/Blueprints/BPI_GameInstance.BPI_GameInstance_C|GetPlayer4Score _asbpi_game_instance))
          (Rendering|Components|TextRender|SetText (Variables|Default|GetTextRender) (Utilities|Text|ToText(Integer) (Variables|/Game/Blueprints/BPI_GameInstance.BPI_GameInstance_C|GetPlayer4Score _asbpi_game_instance))))))))

(event EventBeginPlay
  (Utilities|FlowControl|Delay 0.2)
  (CallFunction|SetVectors)
  (bind _outactors (Actor|GetAllActorsOfClass "/Game/ThirdPersonBP/Blueprints/ThirdPersonCharacter.ThirdPersonCharacter_C"))
  (Variables|Default|SetPlayersRef _outactors)
  (Utilities|Casting|CastToBPI_GameInstance (Game|GetGameInstance))
  (CallFunction|HeightCheck)
  (Utilities|FlowControl|Delay 2.0)
  (Variables|Default|SetLoaded true))

(event EventTick
  (params (DeltaSeconds :type Float%20%28single-precision%29))
  (if (Variables|Default|GetLoaded)
    (CallFunction|MoveUntilInput (Variables|Default|GetMaxHeightVec))))

(fn ConstructionScript)

(fn HeightSet
  (params (Score :type Integer))
  (bind _podiumcube (Variables|Default|GetPodiumCube))
  (bind _returnvalue (Transformation|GetWorldLocation _podiumcube))
  (bind (_x _y _z) (Math|Vector|BreakVector _returnvalue))
  (if (== Score 0)
    (Variables|Default|SetMaxHeightVec "0, 0,-200.000000")
    (Variables|Default|SetPodiumLiftSpeed -1.0)
    (else
      (Variables|Default|SetMaxHeightVec (Math|Vector|MakeVector _x _y (* Score (* _z 2e+01)))))))

(fn SetVectors
  (bind _podiumcube (Variables|Default|GetPodiumCube))
  (bind _returnvalue (Transformation|GetWorldLocation _podiumcube))
  (Variables|Vectors|SetStartVector _returnvalue)
  (Variables|Vectors|Set3rdPlaceVector (+ _returnvalue "0, 0,80.000000"))
  (Variables|Vectors|Set2ndPlaceVector (+ _returnvalue "0, 0,160.000000"))
  (Variables|Vectors|Set1stPlaceVector (+ _returnvalue "0, 0,240.000000")))

(fn CheckPlayerScoring
  (bind _asbpi_game_instance (Utilities|Casting|CastToBPI_GameInstance (Game|GetGameInstance)))
  (Utilities|ScoreChecker (Variables|/Game/Blueprints/BPI_GameInstance.BPI_GameInstance_C|GetPlayer1Score _asbpi_game_instance) (Variables|/Game/Blueprints/BPI_GameInstance.BPI_GameInstance_C|GetPlayer2Score _asbpi_game_instance) (Variables|/Game/Blueprints/BPI_GameInstance.BPI_GameInstance_C|GetPlayer3Score _asbpi_game_instance) (Variables|/Game/Blueprints/BPI_GameInstance.BPI_GameInstance_C|GetPlayer4Score _asbpi_game_instance)
    (:Out
      (Development|PrintString (Utilities|String|ToString(Integer) (Variables|Default|GetLocalScore))))))

(fn MoveUntilInput
  (params (MaxUpVector :type Vector))
  (if (not (Math|Vector|Equal(Vector) (Transformation|GetWorldLocation (Variables|Default|GetPodiumCube)) MaxUpVector 2.0))
    (CallFunction|RaisePodium)))

(fn ScoreCheckandRank
  (bind _asbpi_game_instance (Utilities|Casting|CastToBPI_GameInstance (Game|GetGameInstance)))
  (Utilities|FlowControl|Sequence
    (:then_0
      (if (== (Variables|Default|GetPlayerNumber) 0)
        (Utilities|ScoreChecker (Variables|/Game/Blueprints/BPI_GameInstance.BPI_GameInstance_C|GetPlayer1Score _asbpi_game_instance) (Variables|/Game/Blueprints/BPI_GameInstance.BPI_GameInstance_C|GetPlayer2Score _asbpi_game_instance) (Variables|/Game/Blueprints/BPI_GameInstance.BPI_GameInstance_C|GetPlayer3Score _asbpi_game_instance) (Variables|/Game/Blueprints/BPI_GameInstance.BPI_GameInstance_C|GetPlayer4Score _asbpi_game_instance))))
    (:then_1
      (if (== (Variables|Default|GetPlayerNumber) 1)
        (Utilities|ScoreChecker (Variables|/Game/Blueprints/BPI_GameInstance.BPI_GameInstance_C|GetPlayer2Score _asbpi_game_instance) (Variables|/Game/Blueprints/BPI_GameInstance.BPI_GameInstance_C|GetPlayer1Score _asbpi_game_instance) (Variables|/Game/Blueprints/BPI_GameInstance.BPI_GameInstance_C|GetPlayer3Score _asbpi_game_instance) (Variables|/Game/Blueprints/BPI_GameInstance.BPI_GameInstance_C|GetPlayer4Score _asbpi_game_instance))))
    (:then_2
      (if (== (Variables|Default|GetPlayerNumber) 2)
        (Utilities|ScoreChecker (Variables|/Game/Blueprints/BPI_GameInstance.BPI_GameInstance_C|GetPlayer3Score _asbpi_game_instance) (Variables|/Game/Blueprints/BPI_GameInstance.BPI_GameInstance_C|GetPlayer1Score _asbpi_game_instance) (Variables|/Game/Blueprints/BPI_GameInstance.BPI_GameInstance_C|GetPlayer2Score _asbpi_game_instance) (Variables|/Game/Blueprints/BPI_GameInstance.BPI_GameInstance_C|GetPlayer4Score _asbpi_game_instance))))
    (:then_3
      (if (== (Variables|Default|GetPlayerNumber) 3)
        (Utilities|ScoreChecker (Variables|/Game/Blueprints/BPI_GameInstance.BPI_GameInstance_C|GetPlayer4Score _asbpi_game_instance) (Variables|/Game/Blueprints/BPI_GameInstance.BPI_GameInstance_C|GetPlayer1Score _asbpi_game_instance) (Variables|/Game/Blueprints/BPI_GameInstance.BPI_GameInstance_C|GetPlayer2Score _asbpi_game_instance) (Variables|/Game/Blueprints/BPI_GameInstance.BPI_GameInstance_C|GetPlayer3Score _asbpi_game_instance))))))